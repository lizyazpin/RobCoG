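; PlayerVR_BP is a VR player body that keeps a skeletal mesh under the headset camera of the MCPawn.
; On BeginPlay it caches the first MCPawn's VRCamera, hides the head bone and, after a short delay, matches mesh yaw to the headset once.
; Each Tick offsets the mesh so headSocket tracks the headset horizontally, with world Z pinned to zero.
; Hand-bone hiding nodes are present but unconnected.
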(event `self.ReceiveBeginPlay`
  (bind _outactors (`GameplayStatics.GetAllActorsOfClass` "/Script/UPhysicsBasedMC.MCPawn"))
  (set `self.VRHeadset` (`MCPawn.VRCamera` (`|GetArrayItem` _outactors)))
  (`SkinnedMeshComponent.HideBoneByName` (`self.SkeletalMesh`) "head" "PBO_None")
  (`KismetSystemLibrary.Delay` 0.2)
  (`SceneComponent.K2_SetRelativeRotation` (`self.SkeletalMesh`) (`KismetMathLibrary.MakeRotator` (.roll (`SceneComponent.RelativeRotation` (`self.SkeletalMesh`))) (.pitch (`SceneComponent.RelativeRotation` (`self.SkeletalMesh`))) (.yaw (`SceneComponent.RelativeRotation` (`self.VRHeadset`)))) false false))

(event `self.ReceiveTick`
  (params (DeltaSeconds :type "Float (single-precision)"))
  (bind _skeletalmesh (`self.SkeletalMesh`))
  (`SceneComponent.K2_SetWorldLocation` _skeletalmesh (`KismetMathLibrary.MakeVector` (.x (+ (- (`SceneComponent.K2_GetComponentLocation` (`self.VRHeadset`)) (`SceneComponent.GetSocketLocation` (`self.SkeletalMesh`) "headSocket")) (`SceneComponent.K2_GetComponentLocation` _skeletalmesh))) (.y (+ (- (`SceneComponent.K2_GetComponentLocation` (`self.VRHeadset`)) (`SceneComponent.GetSocketLocation` (`self.SkeletalMesh`) "headSocket")) (`SceneComponent.K2_GetComponentLocation` _skeletalmesh)))) false false))

(fn `UserConstructionScript`)